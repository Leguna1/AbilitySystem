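; BP_TargetDummy is a target dummy character asset that can be targeted and prints combat events as debug text.
; Combatant component events print the damage applied, the hit reaction's instigator and, on death, the killer before the actor destroys itself.
; Targeting functions return the Scene component's world location as the aim point and report it targetable while the Resource component's health is above zero.
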(event `self.ReceiveBeginPlay`)

(event `self.Combatant.OnPayloadReceived`
  (params (Payload :type "AbilityPayload Structure (by ref)") (DamageApplied :type "Float (single-precision)"))
  (`KismetSystemLibrary.PrintString` (`KismetStringLibrary.Conv_DoubleToString` DamageApplied) true true (struct :`R` 1.0 :`B` 0.023582 :`A` 1.0)))

(event `self.Combatant.OnDied`
  (params (Killer :type "Actor Object Reference"))
  (`KismetSystemLibrary.PrintString` (`KismetSystemLibrary.GetDisplayName` Killer) true true (struct :`R` 1.0 :`G` 0.307796 :`A` 1.0))
  (`self.K2_DestroyActor`))

(event `self.Combatant.OnHitReaction`
  (params (Result :type "HitReactionResult Structure (by ref)"))
  (`KismetSystemLibrary.PrintString` (`KismetSystemLibrary.GetDisplayName` (`.Instigator` (break `HitReactionResult` Result)))))

(fn `GetTargetAimLocation`
  (returns (ReturnValue :type "Vector Structure"))
  (return (`SceneComponent.K2_GetComponentLocation` (`self.Scene`))))

(fn `IsTargetable`
  (returns (ReturnValue :type Boolean))
  (return (> (`ResourceComponent.CurrentHealth` (`self.Resource`)) 0.0)))

(fn `UserConstructionScript`)