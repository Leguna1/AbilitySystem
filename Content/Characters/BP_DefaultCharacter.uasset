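; Player character pawn that wires Enhanced Input to component-based combat, inventory and progression systems, and creates the HUD on BeginPlay.
; Movement also feeds the Ability component, while mouse and numbered slot presses and releases go to InputBuffer as gameplay tags.
; Modular body meshes follow the main mesh via leader pose, with equipment meshes registered to Inventory by slot tag.
; Hard-wired keys toggle slow motion, cycle weapons and grant XP, attribute and skill points.
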(event `self.ReceiveBeginPlay`
  (`EnhancedInputSubsystemInterface.AddMappingContext` (subsystem `EnhancedInputLocalPlayerSubsystem`) "/Game/Input/IMC_Default.IMC_Default" 0 (struct))
  (bind _asbp_default_controller (cast `/Game/Characters/BP_DefaultController` (`self.GetController`)))
  (bind _output_get (set `self.As BP Default Controller` _asbp_default_controller))
  (bind _returnvalue (`|CreateWidget` "/Game/Widgets/WB_HUD.WB_HUD_C" _output_get (`self.Combatant`)))
  (set `self.HUD` _returnvalue)
  (`UserWidget.AddToViewport` _returnvalue 0)
  (`self.Set Mesh Ref For Inventory`))

(event `self.ReceiveTick`
  (params (DeltaSeconds :type "Float (single-precision)")))

(event `EnhancedInput|/Game/Input/Actions/IA_Space`
  (params (ActionValue :type Boolean) (ElapsedSeconds :type "Float (double-precision)") (TriggeredSeconds :type "Float (double-precision)") (InputAction :type "InputAction Object Reference" :default "/Game/Input/Actions/IA_Space.IA_Space")))

(event `EnhancedInput|/Game/Input/Actions/IA_Move`
  (params (ActionValue :type "Vector2D Structure") (ElapsedSeconds :type "Float (double-precision)") (TriggeredSeconds :type "Float (double-precision)") (InputAction :type "InputAction Object Reference" :default "/Game/Input/Actions/IA_Move.IA_Move"))
  (:`Triggered`
    (`self.Move` ActionValue)
    (`AbilityComponent.MovementInputReceived` (`self.Ability`) ActionValue))
  (:`Completed`
    (`AbilityComponent.MovementInputReceived` (`self.Ability`) (0.0 0.0))))

(event `EnhancedInput|/Game/Input/Actions/IA_Look`
  (params (ActionValue :type "Vector2D Structure") (ElapsedSeconds :type "Float (double-precision)") (TriggeredSeconds :type "Float (double-precision)") (InputAction :type "InputAction Object Reference" :default "/Game/Input/Actions/IA_Look.IA_Look"))
  (:`Triggered`
    (`self.Look` ActionValue)))

(event `EnhancedInput|/Game/Input/Actions/IA_LeftMouse`
  (params (ActionValue :type Boolean) (ElapsedSeconds :type "Float (double-precision)") (TriggeredSeconds :type "Float (double-precision)") (InputAction :type "InputAction Object Reference" :default "/Game/Input/Actions/IA_LeftMouse.IA_LeftMouse"))
  (:`Started`
    (`InputBufferComponent.HandleInput` (`self.InputBuffer`) (struct :`TagName` "Input.Slot.LMB") ActionValue :!label _label))
  (:`Completed`
    (goto _label)))

(event `EnhancedInput|/Game/Input/Actions/IA_RightMouse`
  (params (ActionValue :type Boolean) (ElapsedSeconds :type "Float (double-precision)") (TriggeredSeconds :type "Float (double-precision)") (InputAction :type "InputAction Object Reference" :default "/Game/Input/Actions/IA_RightMouse.IA_RightMouse"))
  (:`Started`
    (`InputBufferComponent.HandleInput` (`self.InputBuffer`) (struct :`TagName` "Input.Slot.RMB") ActionValue :!label _label_2))
  (:`Completed`
    (goto _label_2)))

(event `Key|Tab`
  (params (Key :type "Key Structure"))
  (:`Pressed`
    (`/Engine/EditorBlueprintResources/StandardMacros.FlipFlop`
      (:`A`
        (`GameplayStatics.SetGlobalTimeDilation` 0.2))
      (:`B`
        (`GameplayStatics.SetGlobalTimeDilation` 1.0)))))

(event `EnhancedInput|/Game/Input/Actions/IA_Slot_1`
  (params (ActionValue :type Boolean) (ElapsedSeconds :type "Float (double-precision)") (TriggeredSeconds :type "Float (double-precision)") (InputAction :type "InputAction Object Reference" :default "/Game/Input/Actions/IA_Slot_1.IA_Slot_1"))
  (:`Started`
    (`InputBufferComponent.HandleInput` (`self.InputBuffer`) (struct :`TagName` "Input.Slot.1") ActionValue :!label _label_3))
  (:`Completed`
    (goto _label_3)))

(event `EnhancedInput|/Game/Input/Actions/IA_Slot_6`
  (params (ActionValue :type Boolean) (ElapsedSeconds :type "Float (double-precision)") (TriggeredSeconds :type "Float (double-precision)") (InputAction :type "InputAction Object Reference" :default "/Game/Input/Actions/IA_Slot_6.IA_Slot_6"))
  (:`Started`
    (`InputBufferComponent.HandleInput` (`self.InputBuffer`) (struct :`TagName` "Input.Slot.6") ActionValue :!label _label_4))
  (:`Completed`
    (goto _label_4)))

(event `EnhancedInput|/Game/Input/Actions/IA_Slot_7`
  (params (ActionValue :type Boolean) (ElapsedSeconds :type "Float (double-precision)") (TriggeredSeconds :type "Float (double-precision)") (InputAction :type "InputAction Object Reference" :default "/Game/Input/Actions/IA_Slot_7.IA_Slot_7"))
  (:`Started`
    (`InputBufferComponent.HandleInput` (`self.InputBuffer`) (struct :`TagName` "Input.Slot.7") ActionValue :!label _label_5))
  (:`Completed`
    (goto _label_5)))

(event `EnhancedInput|/Game/Input/Actions/IA_Slot_2`
  (params (ActionValue :type Boolean) (ElapsedSeconds :type "Float (double-precision)") (TriggeredSeconds :type "Float (double-precision)") (InputAction :type "InputAction Object Reference" :default "/Game/Input/Actions/IA_Slot_2.IA_Slot_2"))
  (:`Started`
    (`InputBufferComponent.HandleInput` (`self.InputBuffer`) (struct :`TagName` "Input.Slot.2") ActionValue :!label _label_6))
  (:`Completed`
    (goto _label_6)))

(event `EnhancedInput|/Game/Input/Actions/IA_Slot_3`
  (params (ActionValue :type Boolean) (ElapsedSeconds :type "Float (double-precision)") (TriggeredSeconds :type "Float (double-precision)") (InputAction :type "InputAction Object Reference" :default "/Game/Input/Actions/IA_Slot_3.IA_Slot_3"))
  (:`Started`
    (`InputBufferComponent.HandleInput` (`self.InputBuffer`) (struct :`TagName` "Input.Slot.3") ActionValue :!label _label_7))
  (:`Completed`
    (goto _label_7)))

(event `EnhancedInput|/Game/Input/Actions/IA_Slot_8`
  (params (ActionValue :type Boolean) (ElapsedSeconds :type "Float (double-precision)") (TriggeredSeconds :type "Float (double-precision)") (InputAction :type "InputAction Object Reference" :default "/Game/Input/Actions/IA_Slot_8.IA_Slot_8"))
  (:`Started`
    (`InputBufferComponent.HandleInput` (`self.InputBuffer`) (struct :`TagName` "Input.Slot.8") ActionValue :!label _label_8))
  (:`Completed`
    (goto _label_8)))

(event `EnhancedInput|/Game/Input/Actions/IA_Slot_4`
  (params (ActionValue :type Boolean) (ElapsedSeconds :type "Float (double-precision)") (TriggeredSeconds :type "Float (double-precision)") (InputAction :type "InputAction Object Reference" :default "/Game/Input/Actions/IA_Slot_4.IA_Slot_4"))
  (:`Started`
    (`InputBufferComponent.HandleInput` (`self.InputBuffer`) (struct :`TagName` "Input.Slot.4") ActionValue :!label _label_9))
  (:`Completed`
    (goto _label_9)))

(event `EnhancedInput|/Game/Input/Actions/IA_Slot_9`
  (params (ActionValue :type Boolean) (ElapsedSeconds :type "Float (double-precision)") (TriggeredSeconds :type "Float (double-precision)") (InputAction :type "InputAction Object Reference" :default "/Game/Input/Actions/IA_Slot_9.IA_Slot_9"))
  (:`Started`
    (`InputBufferComponent.HandleInput` (`self.InputBuffer`) (struct :`TagName` "Input.Slot.9") ActionValue :!label _label_10))
  (:`Completed`
    (goto _label_10)))

(event `EnhancedInput|/Game/Input/Actions/IA_Slot_5`
  (params (ActionValue :type Boolean) (ElapsedSeconds :type "Float (double-precision)") (TriggeredSeconds :type "Float (double-precision)") (InputAction :type "InputAction Object Reference" :default "/Game/Input/Actions/IA_Slot_5.IA_Slot_5"))
  (:`Started`
    (`InputBufferComponent.HandleInput` (`self.InputBuffer`) (struct :`TagName` "Input.Slot.5") ActionValue :!label _label_11))
  (:`Completed`
    (goto _label_11)))

(event `EnhancedInput|/Game/Input/Actions/IA_Slot_0`
  (params (ActionValue :type Boolean) (ElapsedSeconds :type "Float (double-precision)") (TriggeredSeconds :type "Float (double-precision)") (InputAction :type "InputAction Object Reference" :default "/Game/Input/Actions/IA_Slot_0.IA_Slot_0"))
  (:`Started`
    (`InputBufferComponent.HandleInput` (`self.InputBuffer`) (struct :`TagName` "Input.Slot.0") ActionValue :!label _label_12))
  (:`Completed`
    (goto _label_12)))

(event `Key|NumPadZero`
  (params (Key :type "Key Structure"))
  (:`Pressed`
    (`WeaponManagerComponent.CycleWeapon` (`self.WeaponManager`) 1)))

(event `Key|NumPadOne`
  (params (Key :type "Key Structure"))
  (:`Pressed`
    (`ExperienceComponent.AddExperience` (`self.Experience`) 100)))

(event `Key|NumPadThree`
  (params (Key :type "Key Structure"))
  (:`Pressed`
    (`AttributeComponent.AddAttributePoints` (`self.Attribute`) 5)))

(event `Key|NumPadTwo`
  (params (Key :type "Key Structure"))
  (:`Pressed`
    (`SkillTreeComponent.AddSkillPoints` (`self.SkillTree`) 5)))

(fn `GetTargetAimLocation`
  (returns (ReturnValue :type "Vector Structure"))
  (return (`self.K2_GetActorLocation`)))

(fn `IsTargetable`
  (returns (ReturnValue :type Boolean))
  (return true))

(fn `Look`
  (params (`Action Axis` :type "Vector2D Structure"))
  (`self.AddControllerYawInput` `Action Axis_X`)
  (`self.AddControllerPitchInput` `Action Axis_Y`))

(fn `Move`
  (params (`Action Axis` :type "Vector2D Structure"))
  (bind (_returnvalue_roll _returnvalue_pitch _returnvalue_yaw) (`KismetMathLibrary.BreakRotator` (`self.GetControlRotation`)))
  (bind (_returnvalue_roll_2 _returnvalue_pitch_2 _returnvalue_yaw_2) (`KismetMathLibrary.BreakRotator` (`self.GetControlRotation`)))
  (`self.AddMovementInput` (`KismetMathLibrary.GetRightVector` (`KismetMathLibrary.MakeRotator` _returnvalue_roll_2 0.0 _returnvalue_yaw_2)) `Action Axis_X`)
  (`self.AddMovementInput` (`KismetMathLibrary.GetForwardVector` (`KismetMathLibrary.MakeRotator` 0.0 0.0 _returnvalue_yaw)) `Action Axis_Y`))

(fn `Set Mesh Ref For Inventory`
  (`|ExecutionSequence`
    (:`then_0`
      (bind _structout (setmembers `EquipmentMeshBinding` :`StructRef` (make `EquipmentMeshBinding` (struct :`TagName` "Equipment.Slot.Head") (`self.Helmet`)))))
    (:`then_1`
      (bind _structout_2 (setmembers `EquipmentMeshBinding` :`StructRef` (make `EquipmentMeshBinding` (struct :`TagName` "Equipment.Slot.Feet") (`self.Feet_Slot1`)))))
    (:`then_2`
      (bind _structout_3 (setmembers `EquipmentMeshBinding` :`StructRef` (make `EquipmentMeshBinding` (struct :`TagName` "Equipment.Slot.Chest") (`self.Torso_Slot1`)))))
    (:`then_3`
      (bind _structout_4 (setmembers `EquipmentMeshBinding` :`StructRef` (make `EquipmentMeshBinding` (struct :`TagName` "Equipment.Slot.Legs") (`self.Legs_Slot1`)))))
    (:`then_4`
      (bind _structout_5 (setmembers `EquipmentMeshBinding` :`StructRef` (make `EquipmentMeshBinding` (struct :`TagName` "Equipment.Slot.Hands") (`self.Hands_Slot1`)))))
    (:`then_5`
      (bind _structout_6 (setmembers `EquipmentMeshBinding` :`StructRef` (make `EquipmentMeshBinding` (struct :`TagName` "Equipment.Slot.Back") (`self.Back`)))))
    (:`then_6`
      (bind _structout_7 (setmembers `EquipmentMeshBinding` :`StructRef` (make `EquipmentMeshBinding` (struct :`TagName` "Equipment.Slot.Waist") (`self.Legs_Slot2`))))))
  (`InventoryComponent.RegisterEquipmentMeshes` (`self.Inventory`) (`|MakeArray` _structout _structout_2 _structout_3 _structout_4 _structout_5 _structout_6 _structout_7)))

(fn `Toggle Mouse Cursor`
  (params (`Show Mouse Cursor` :type Boolean))
  (bind _as_bp_default_controller (`self.As BP Default Controller`))
  (bind _as_bp_default_controller_2 (`self.As BP Default Controller`))
  (if `Show Mouse Cursor`
    (set `PlayerController.bShowMouseCursor` true _as_bp_default_controller)
    (`WidgetBlueprintLibrary.SetInputMode_GameAndUIEx` _as_bp_default_controller (`self.HUD`))
    (else
      (set `PlayerController.bShowMouseCursor` false _as_bp_default_controller_2)
      (`WidgetBlueprintLibrary.SetInputMode_GameOnly` _as_bp_default_controller_2))))

(fn `UserConstructionScript`
  (`SkinnedMeshComponent.SetLeaderPoseComponent` (`self.Hands`) (`self.Mesh`) false false)
  (`SkinnedMeshComponent.SetLeaderPoseComponent` (`self.Torso`) (`self.Mesh`) false false)
  (`SkinnedMeshComponent.SetLeaderPoseComponent` (`self.Arms`) (`self.Mesh`) false false)
  (`SkinnedMeshComponent.SetLeaderPoseComponent` (`self.Legs`) (`self.Mesh`) false false)
  (`SkinnedMeshComponent.SetLeaderPoseComponent` (`self.Feet`) (`self.Mesh`) false false)
  (`SkinnedMeshComponent.SetLeaderPoseComponent` (`self.Legs_Slot1`) (`self.Mesh`) false false)
  (`SkinnedMeshComponent.SetLeaderPoseComponent` (`self.Helmet`) (`self.Mesh`) false false)
  (`SkinnedMeshComponent.SetLeaderPoseComponent` (`self.Feet_Slot1`) (`self.Mesh`) false false)
  (`SkinnedMeshComponent.SetLeaderPoseComponent` (`self.Legs_Slot2`) (`self.Mesh`) false false)
  (`SkinnedMeshComponent.SetLeaderPoseComponent` (`self.Hands_Slot1`) (`self.Mesh`) false false)
  (`SkinnedMeshComponent.SetLeaderPoseComponent` (`self.Torso_Slot1`) (`self.Mesh`) false false)
  (`SkinnedMeshComponent.SetLeaderPoseComponent` (`self.Back`) (`self.Mesh`) false false)
  (`SkinnedMeshComponent.SetLeaderPoseComponent` (`self.Legs_Slot1`) (`self.Mesh`) false false))