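; Golem enemy character that can be targeted while its current Health is above zero.
; On BeginPlay it runs the parent logic and binds a handler to its combatant component's payload-received event, which only prints the damage applied.
; Targeting queries read Health from the resource component and return the world location of an AimLocation component as the aim point.
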(event `self.ReceiveBeginPlay`
  (`parent.ReceiveBeginPlay`)
  (add `CombatantComponent.OnPayloadReceived` (`self.GetCombatantComponent`) (`|CreateDelegate` :!event `BP_Enemy_Golem_AutoGenFunc`)))

(fn `BP_Enemy_Golem_AutoGenFunc`
  (params (Payload :type "AbilityPayload Structure (by ref)") (DamageApplied :type "Float (single-precision)"))
  (`KismetSystemLibrary.PrintString` (`KismetStringLibrary.Conv_DoubleToString` DamageApplied))
  (return))

(fn `GetTargetAimLocation`
  (returns (ReturnValue :type "Vector Structure"))
  (return (`SceneComponent.K2_GetComponentLocation` (`self.Aim Location`))))

(fn `IsTargetable`
  (returns (ReturnValue :type Boolean))
  (return (> (`ResourceComponent.GetResourceValue` (`self.GetResourceComponent`) "Health" "Current") 0.0)))

(fn `UserConstructionScript`)